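; Drone spawner that runs endless waves by spawning straight-line, V or random-cluster formations at its own location.
; Tick jitters the spawner along X within XRange around its start, so formation placement varies; the RandomX inputs go unused.
; ChooseFormation shows a fading WaveUI, picks a weighted random formation or none, and re-arms itself on a shrinking timer.
; Each wave allows WaveNumber + 2 picks, then increments and sets a longer randomised delay.
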(event `self.ReceiveBeginPlay`
  (bind _output_get (set `self.SpawnerTransform` (`self.GetTransform`)))
  (set `self.XInitial` (.x (.location _output_get)))
  (set `self.Timer` 25.0)
  (set `self.TimerDecrease` 10.0)
  (`self.Choose_Formation`))

(event `self.ReceiveTick`
  (params (DeltaSeconds :type "Float (single-precision)"))
  (bind _returnvalue (`self.K2_GetActorLocation`))
  (bind _xrange (`self.XRange`))
  (`self.K2_SetActorLocation` (`KismetMathLibrary.VInterpTo` _returnvalue (`KismetMathLibrary.MakeVector` (+ (`self.XInitial`) (`KismetMathLibrary.RandomFloatInRange` (* _xrange -1.0) _xrange)) (.y _returnvalue) (.z _returnvalue)) DeltaSeconds 60.0))
  (set `self.SpawnerTransform` (`self.GetTransform`))
  (if (> (`self.WaveNumber`) 3)
    _))

(fn `Choose_Formation`
  (bind _xrange (`self.XRange`))
  (bind _wavenumber (`self.WaveNumber`))
  (bind _returnvalue (`KismetMathLibrary.FClamp` (+ (* (`self.Timer`) (`KismetMathLibrary.RandomFloatInRange` 1.5 2.0)) (`KismetMathLibrary.RandomFloatInRange` 10.0 30.0)) 30.0 500.0))
  (bind _returnvalue_2 (+ (`KismetMathLibrary.RandomFloatInRange` (* _xrange -1.0) _xrange) (.x (.location (`self.SpawnerTransform`)))))
  (bind _returnvalue_3 (`|CreateWidget` "/Game/UI/WaveUI.WaveUI_C"))
  (`UserWidget.AddToViewport` _returnvalue_3 0)
  (`UserWidget.PlayAnimation` _returnvalue_3 (`/Game/UI/WaveUI.TextFade` _returnvalue_3) 0.0 1 "Forward" 1.0 false)
  (if (>= (`self.DroneFormationSpawns`) (+ _wavenumber 2))
    (`KismetSystemLibrary.PrintString` (`KismetStringLibrary.BuildString_Int` "" "Wave " _wavenumber " Complete"))
    (set `self.DroneFormationSpawns` 0)
    (set `self.WaveNumber` (+ _wavenumber 1))
    (`KismetSystemLibrary.K2_SetTimer` null "Choose Formation" _returnvalue)
    (`KismetSystemLibrary.PrintString` (`KismetStringLibrary.BuildString_Double` "" "Time until next Wave:" _returnvalue) true true (struct :`G` 0.66 :`B` 1.0 :`A` 1.0) 8.0)
    (else
      (switch `int` (`KismetMathLibrary.RandomIntegerInRange` 0 5)
        (:`Default`
          (`KismetSystemLibrary.PrintString` "Spawned no formation" :!label _label))
        (:`0`
          (`self.Formation_Straight` _returnvalue_2 :!label _label_2))
        (:`1`
          (goto _label_2))
        (:`2`
          (`self.Formation_V` _returnvalue_2 :!label _label_3))
        (:`3`
          (goto _label_3))
        (:`4`
          (`self.Formation_Cluster` _returnvalue_2))
        (:`5`
          (goto _label)))
      (bind _output_get (set `self.DroneFormationSpawns` (+ (`self.DroneFormationSpawns`) 1)))
      (`KismetSystemLibrary.PrintString` (`KismetStringLibrary.BuildString_Int` (`KismetStringLibrary.BuildString_Int` "" "Wave Number:" _wavenumber) "Spawn Number:" _output_get) true true (struct :`G` 0.66 :`B` 1.0 :`A` 1.0) 8.0)
      (if (`KismetSystemLibrary.K2_IsTimerActive` null "Choose_Formation")
        (`KismetSystemLibrary.K2_ClearTimer` null "Choose_Formation")
        (`KismetSystemLibrary.K2_SetTimer` null "Choose_Formation" (`self.Timer`) true)
        (bind _output_get_2 (set `self.Timer` (`KismetMathLibrary.FClamp` (* (`self.Timer`) 0.95) (`KismetMathLibrary.RandomFloatInRange` 1.0 10.0) 500.0)))
        (`KismetSystemLibrary.PrintString` (`KismetStringLibrary.Conv_DoubleToString` _output_get_2))
        (`KismetSystemLibrary.PrintString` "Timer:")
        (else
          (`KismetSystemLibrary.K2_SetTimer` null "Choose_Formation" (`self.Timer`) true))))))

(fn `Formation_Cluster`
  (params (RandomX :type "Float (double-precision)"))
  (bind _spawnertransform (`self.SpawnerTransform`))
  ; Spawns a cluster of drones, placed randomly within a certain distance of the spawner
  (for _ (range 24)
    (`|SpawnActorFromClass` "/Game/Drones/Drone.Drone_C" (`KismetMathLibrary.MakeTransform` (`KismetMathLibrary.MakeVector` (+ (.x (.location _spawnertransform)) (`KismetMathLibrary.RandomIntegerInRange` -2000 2000)) (.y (.location _spawnertransform)) (+ (.z (.location _spawnertransform)) (`KismetMathLibrary.RandomIntegerInRange` -2000 2000))) (struct) (2.0 2.0 2.0)) "Undefined" "MultiplyWithRoot" null null))
  (`KismetSystemLibrary.PrintString` "Cluster formation spawned"))

(fn `Formation_Straight`
  (params (RandomX :type "Float (double-precision)"))
  (bind _spawnertransform (`self.SpawnerTransform`))
  ; Spawns 15 drones along the x axis 450px apart
  (for _index (range 15)
    (`|SpawnActorFromClass` "/Game/Drones/Drone.Drone_C" (`KismetMathLibrary.MakeTransform` (`KismetMathLibrary.MakeVector` (+ (* _index 450) (.x (.location _spawnertransform))) (.y (.location _spawnertransform)) (.z (.location _spawnertransform))) (struct) (2.0 2.0 2.0)) "Undefined" "MultiplyWithRoot" null null))
  (`KismetSystemLibrary.PrintString` "Straight formation spawned"))

(fn `Formation_V`
  (params (RandomX :type "Float (double-precision)"))
  (bind _spawnertransform (`self.SpawnerTransform`))
  ; Spawns drones in a V shape
  (`|SpawnActorFromClass` "/Game/Drones/Drone.Drone_C" (`self.SpawnerTransform`) "Undefined" "MultiplyWithRoot" null null) ; Center point of V shape
  (for _index (range 7)
    (bind _returnvalue (* _index 550))
    (bind _returnvalue_2 (+ _returnvalue (.z (.location _spawnertransform))))
    ;; Left side of 'V'
    (`|SpawnActorFromClass` "/Game/Drones/Drone.Drone_C" (`KismetMathLibrary.MakeTransform` (`KismetMathLibrary.MakeVector` (+ _returnvalue (.x (.location _spawnertransform))) (.y (.location _spawnertransform)) _returnvalue_2) (struct) (2.0 2.0 2.0)) "Undefined" "MultiplyWithRoot" null null)
    ;; Right side of 'V'
    (`|SpawnActorFromClass` "/Game/Drones/Drone.Drone_C" (`KismetMathLibrary.MakeTransform` (`KismetMathLibrary.MakeVector` (- (.x (.location _spawnertransform)) _returnvalue) (.y (.location _spawnertransform)) _returnvalue_2) (struct) (2.0 2.0 2.0)) "Undefined" "MultiplyWithRoot" null null))
  (`KismetSystemLibrary.PrintString` "V formation spawned"))

(fn `UserConstructionScript`)