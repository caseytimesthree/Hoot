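; BP_Perch is a clickable landing spot for the owl player.
; Clicking its Capsule casts the player pawn to BP_Owl, sets IsLanding and hands it the capsule's world location as PerchTarget, printing debug messages along the way.
; BeginPlay pushes the perch sprite behind others with a negative translucent sort priority, while the overlap check against the player has no effect.
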(event `self.ReceiveBeginPlay`
  (`PrimitiveComponent.SetTranslucentSortPriority` (`self.PerchSprite`) -1))

(event `self.ReceiveActorBeginOverlap`
  (params (OtherActor :type "Actor Object Reference"))
  (if (== OtherActor (`GameplayStatics.GetPlayerPawn` 0))
    _))

(event `self.Capsule.OnClicked`
  (params (TouchedComponent :type "PrimitiveComponent Object Reference") (ButtonPressed :type "Key Structure"))
  (`KismetSystemLibrary.PrintString` "Perch Clicked")
  (bind _asbp_owl (cast `/Game/Owl/BP_Owl` (`GameplayStatics.GetPlayerPawn` 0)))
  (set `/Game/Owl/BP_Owl.IsLanding` true _asbp_owl)
  (`KismetSystemLibrary.PrintString` "Owl is Landing")
  (set `/Game/Owl/BP_Owl.PerchTarget` (`SceneComponent.K2_GetComponentLocation` TouchedComponent) _asbp_owl))

(fn `UserConstructionScript`)