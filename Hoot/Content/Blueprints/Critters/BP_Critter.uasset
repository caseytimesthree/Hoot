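; Prey critter that the player's owl catches by diving at it when clicked, then carries, eats or throws.
; On overlap it follows the owl, and X eats it, incrementing the controller's eaten count.
; Holding space swings it in an accelerating X/Z orbit; release tosses it toward the cursor at a speed scaled by hold time.
; Tick drives follow, orbit and toss, while a random lifetime timer despawns critters not being carried.
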(event `self.ReceiveTick`
  (params (DeltaSeconds :type "Float (single-precision)"))
  (if (`self.isFollowing`)
    (if (`self.SpaceHeld`)
      (`self.Orbit` DeltaSeconds)
      (else
        (`self.K2_SetActorLocation` (+ (`self.K2_GetActorLocation` (`GameplayStatics.GetPlayerPawn` 0)) (50.0 50.0 -10.0)) true) ; Set new location
      ))
    (elif (`self.isTossed`)
      (`self.Toss` DeltaSeconds)
      (set `self.isFollowing` false))))

(event `self.Box.OnClicked`
  (params (TouchedComponent :type "PrimitiveComponent Object Reference") (ButtonPressed :type "Key Structure"))
  ; Clicked on
  (if (not (`self.isFollowing`))
    (bind _asbp_owl (cast `/Game/Owl/BP_Owl` (`GameplayStatics.GetPlayerPawn` 0)))
    (set `/Game/Owl/BP_Owl.isDiving` true _asbp_owl)
    (set `/Game/Owl/BP_Owl.CritterTarget` (`self.K2_GetActorLocation`) _asbp_owl)))

(event `self.ReceiveBeginPlay`
  (bind (_returnvalue_x _returnvalue_y _returnvalue_z) (`KismetMathLibrary.BreakVector` (`self.K2_GetActorLocation`)))
  (`self.EnableInput` (`GameplayStatics.GetPlayerController` 0))
  (if (`KismetMathLibrary.RandomBool`)
    (`AudioComponent.Play` (`self.squeak`) 0.8))
  ; Lifetime
  (bind _output_get (set `self.Lifetime` (* (`KismetMathLibrary.RandomFloat`) 5.0)))
  (`KismetSystemLibrary.K2_SetTimer` null "DestroySelf" _output_get)
  ; Grabbable
  (`self.K2_SetActorLocation` (`KismetMathLibrary.MakeVector` _returnvalue_x 100.0 _returnvalue_z))
  (`self.SetUpGrabbable`)
  (add `self.OnSpacebarPressed` (delegate `SpacebarPressed`))
  (add `self.OnSpacebarReleased` (delegate `SpacebarReleased`)))

(event `SpacebarReleased`
  ; Grabbable
  (if (`self.isFollowing`)
    (`self.TossSetUp`)
    (set `self.isFollowing` false)))

(event `SpacebarPressed`
  ; Grabbable
  (set `self.PressStartTime` (`KismetSystemLibrary.GetGameTimeInSeconds`))
  (set `self.SpaceHeld` true))

(event `Key|X`
  (params (Key :type "Key Structure"))
  ; Eat
  (:`Pressed`
    (if (`self.isFollowing`) :!label _label
      (`KismetSystemLibrary.PrintString` "Critter Eaten")
      (bind _ashoot_player_controller (cast `/Game/Owl/Hoot_PlayerController` (`GameplayStatics.GetPlayerController` 0)))
      (set `/Game/Owl/Hoot_PlayerController.CrittersEaten` (+ (`/Game/Owl/Hoot_PlayerController.CrittersEaten` _ashoot_player_controller) 1) _ashoot_player_controller)
      (`self.K2_DestroyActor`)
      (bind _asbp_owl (cast `/Game/Owl/BP_Owl` (`GameplayStatics.GetPlayerPawn` 0)))
      (`/Game/Owl/BP_Owl.Eat` _asbp_owl)))
  (:`Released`
    (goto _label)))

(event `self.Box.OnComponentBeginOverlap`
  (params (OverlappedComponent :type "PrimitiveComponent Object Reference") (OtherActor :type "Actor Object Reference") (OtherComp :type "PrimitiveComponent Object Reference") (OtherBodyIndex :type Integer) (bFromSweep :type Boolean) (SweepResult :type "HitResult Structure (by ref)"))
  ; When Owl Touches
  (if (== OtherActor (`GameplayStatics.GetPlayerPawn` 0))
    (bind _asbp_owl (cast `/Game/Owl/BP_Owl` (`GameplayStatics.GetPlayerPawn` 0)))
    (set `/Game/Owl/BP_Owl.isDiving` false _asbp_owl)
    (`SceneComponent.SetVisibility` (`self.DistortionsFX`) false true) ; Show Critter Caught Sprite
    (`SceneComponent.SetVisibility` (`self.Caught`) true false) ; Show Critter Caught Sprite
    (set `self.isFollowing` true) ; Attach the object to the player when it is clicked on
    (set `self.SpaceHeld` false)
    (set `self.OrbitSpeed` 0.0)))

(event `DestroySelf`
  ; Evade Capture
  (if (not (`self.isFollowing`))
    (`KismetSystemLibrary.Delay` 4.0)
    (`self.K2_DestroyActor`)))

(fn `Orbit`
  (params (DeltaTime :type "Float (double-precision)"))
  (bind (_returnvalue_x _returnvalue_y _returnvalue_z) (`KismetMathLibrary.BreakVector` (`self.K2_GetActorLocation` (`GameplayStatics.GetPlayerPawn` 0))))
  (set `self.OrbitSpeed` (+ (`self.OrbitSpeed`) 10.0))
  (set `self.CurrentAngle` (+ (* (`self.OrbitSpeed`) DeltaTime) (`self.CurrentAngle`)))
  (`self.K2_SetActorLocation` (`KismetMathLibrary.MakeVector` (+ (* (`KismetMathLibrary.DegCos` (`self.CurrentAngle`)) (`self.OrbitRadius`)) _returnvalue_x) 0.0 (+ (* (`KismetMathLibrary.DegSin` (`self.CurrentAngle`)) (`self.OrbitRadius`)) _returnvalue_z))))

(fn `SetUpGrabbable`
  (`SceneComponent.SetVisibility` (`self.Caught`) false false) ; No outline on startup
  (set `self.isFollowing` false) ; Not following on startup
  (`self.EnableInput` (`GameplayStatics.GetPlayerController` 0))
  (`self.K2_SetActorLocation` (`KismetMathLibrary.MakeVector` (.x (`self.K2_GetActorLocation`)) (.y (`self.K2_GetActorLocation`)) (.z (`self.K2_GetActorLocation`))) false true))

(fn `Toss`
  (params (DeltaTime :type "Float (double-precision)"))
  (bind (_returnvalue_x _returnvalue_y _returnvalue_z) (`KismetMathLibrary.BreakVector` (+ (* (`self.MoveSpeed`) (`self.MoveDirection`) DeltaTime) (`self.K2_GetActorLocation`))))
  (`self.K2_SetActorLocation` (`KismetMathLibrary.MakeVector` _returnvalue_x 0.0 _returnvalue_z)))

(fn `TossSetUp`
  (set `self.TimeHeld` (- (`KismetSystemLibrary.GetGameTimeInSeconds`) (`self.PressStartTime`)))
  (set `self.SpaceHeld` false)
  (set `self.MouseLocation` (`.Location` (`GameplayStatics.BreakHitResult` (`PlayerController.GetHitResultUnderCursorByChannel` (`GameplayStatics.GetPlayerController` 0) "TraceTypeQuery1" true))))
  (set `self.MoveDirection` (`KismetMathLibrary.Normal` (- (`self.MouseLocation`) (`self.K2_GetActorLocation`))))
  (set `self.MoveSpeed` (* (`self.TimeHeld`) 1000.0))
  (if (`self.isFollowing`)
    (set `self.isTossed` true)
    (set `self.isFollowing` false)))

(fn `UserConstructionScript`)