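; Grabbable actor that attaches to the player when clicked, swings around them while Space is held, and is thrown on release.
; Tick drives follow-at-offset, an accelerating sine/cosine orbit in the X-Z plane, or straight-line toss movement.
; Release aims at the cursor hit point, with speed scaled by hold time.
; Cursor hover swaps normal and outlined components for highlighting.
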(event `self.ReceiveTick`
  (params (DeltaSeconds :type "Float (single-precision)"))
  (if (`self.isFollowing`)
    (if (`self.SpaceHeld`)
      (`self.Orbit` DeltaSeconds)
      (else
        (`self.K2_SetActorLocation` (+ (`self.K2_GetActorLocation` (`GameplayStatics.GetPlayerPawn` 0)) (50.0 50.0 -10.0)) true) ; Set new location
      ))
    (elif (`self.isTossed`)
      (`self.Toss` DeltaSeconds)
      (set `self.isFollowing` false))))

(event `self.ReceiveBeginPlay`
  (bind (_returnvalue_x _returnvalue_y _returnvalue_z) (`KismetMathLibrary.BreakVector` (`self.K2_GetActorLocation`)))
  (`self.K2_SetActorLocation` (`KismetMathLibrary.MakeVector` _returnvalue_x 0.0 _returnvalue_z))
  (`self.SetUpGrabbable`)
  (add `self.OnSpacebarPressed` (delegate `SpacebarPressed`))
  (add `self.OnSpacebarReleased` (delegate `SpacebarReleased`)))

(event `SpacebarReleased`
  (if (`self.isFollowing`)
    (`self.TossSetUp`)
    (set `self.isFollowing` false)))

(event `SpacebarPressed`
  (set `self.PressStartTime` (`KismetSystemLibrary.GetGameTimeInSeconds`))
  (set `self.SpaceHeld` true))

(event `self.ReceiveActorEndCursorOver`
  (`SceneComponent.SetVisibility` (`self.Outlined`) false false) ; Turn off normal
  (`SceneComponent.SetVisibility` (`self.Normal`) true false) ; Turn on normal
)

(event `self.ReceiveActorBeginCursorOver`
  (`SceneComponent.SetVisibility` (`self.Outlined`) true false) ; Turn on outline
  (`SceneComponent.SetVisibility` (`self.Normal`) false false) ; Turn off outline
)

(event `self.ReceiveActorOnClicked`
  (params (ButtonPressed :type "Key Structure"))
  (set `self.isFollowing` true) ; Attach the object to the player when it is clicked on
  (set `self.SpaceHeld` false)
  (set `self.OrbitSpeed` 0.0))

(fn `Orbit`
  (params (DeltaTime :type "Float (double-precision)"))
  (bind (_returnvalue_x _returnvalue_y _returnvalue_z) (`KismetMathLibrary.BreakVector` (`self.K2_GetActorLocation` (`GameplayStatics.GetPlayerPawn` 0))))
  (set `self.OrbitSpeed` (+ (`self.OrbitSpeed`) 10.0))
  (set `self.CurrentAngle` (+ (* (`self.OrbitSpeed`) DeltaTime) (`self.CurrentAngle`)))
  (`self.K2_SetActorLocation` (`KismetMathLibrary.MakeVector` (+ (* (`KismetMathLibrary.DegCos` (`self.CurrentAngle`)) (`self.OrbitRadius`)) _returnvalue_x) 0.0 (+ (* (`KismetMathLibrary.DegSin` (`self.CurrentAngle`)) (`self.OrbitRadius`)) _returnvalue_z))))

(fn `SetUpGrabbable`
  (`SceneComponent.SetVisibility` (`self.Outlined`) false false) ; No outline on startup
  (set `self.isFollowing` false) ; Not following on startup
  (`self.EnableInput` (`GameplayStatics.GetPlayerController` 0))
  (`self.K2_SetActorLocation` (`KismetMathLibrary.MakeVector` (.x (`self.K2_GetActorLocation`)) (.y (`self.K2_GetActorLocation`)) (.z (`self.K2_GetActorLocation`))) false true))

(fn `Toss`
  (params (DeltaTime :type "Float (double-precision)"))
  (bind (_returnvalue_x _returnvalue_y _returnvalue_z) (`KismetMathLibrary.BreakVector` (+ (* (`self.MoveSpeed`) (`self.MoveDirection`) DeltaTime) (`self.K2_GetActorLocation`))))
  (`self.K2_SetActorLocation` (`KismetMathLibrary.MakeVector` _returnvalue_x 0.0 _returnvalue_z)))

(fn `TossSetUp`
  (set `self.TimeHeld` (- (`KismetSystemLibrary.GetGameTimeInSeconds`) (`self.PressStartTime`)))
  (set `self.SpaceHeld` false)
  (set `self.MouseLocation` (`.Location` (`GameplayStatics.BreakHitResult` (`PlayerController.GetHitResultUnderCursorByChannel` (`GameplayStatics.GetPlayerController` 0) "TraceTypeQuery1" true))))
  (set `self.MoveDirection` (`KismetMathLibrary.Normal` (- (`self.MouseLocation`) (`self.K2_GetActorLocation`))))
  (set `self.MoveSpeed` (* (`self.TimeHeld`) 1000.0))
  (if (`self.isFollowing`)
    (set `self.isTossed` true)
    (set `self.isFollowing` false)))

(fn `UserConstructionScript`)