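; BP_Building is a destructible 2D sprite building that hosts a perch and spawns critters.
; On BeginPlay it places a BP_Perch atop the intact sprite, then loops, spawning a BP_Critter after random delays.
; HootHeard spawns an extra critter immediately.
; Depleted health swaps sprites, plays the destruction flipbook with smoke and explosion emitters, then destroys the actor when the animation ends.
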(event `self.ReceiveAnyDamage`
  (params (Damage :type "Float (single-precision)") (DamageType :type "DamageType Object Reference") (InstigatedBy :type "Controller Object Reference") (DamageCauser :type "Actor Object Reference"))
  (bind _remnant_sprite (`self.Remnant_Sprite`))
  (bind _destroyanimation (`self.DestroyAnimation`))
  (bind _destroyedemittersize (`self.DestroyedEmitterSize`))
  (bind _location (.location (`self.GetTransform`)))
  (bind _rotation (.rotation (`self.GetTransform`)))
  (bind _returnvalue (* (`KismetMathLibrary.MakeVector` _destroyedemittersize 0.0 _destroyedemittersize) (.scale (`self.GetTransform`))))
  ; Receive Damage
  (`KismetSystemLibrary.PrintString` "Building Damage Received")
  (bind _output_get (set `self.Health` (- (`self.Health`) Damage)))
  (if (<= (`self.Health`) 0.0)
    (`KismetSystemLibrary.PrintString` "Building Destroy Triggered")
    ; Remove Intact Sprite
    (`SceneComponent.SetVisibility` (`self.Intact_Sprite`) false false)
    ; Play Destroy Animation
    (`SceneComponent.SetHiddenInGame` _destroyanimation false false)
    (`PaperFlipbookComponent.PlayFromStart` _destroyanimation)
    ; Smoke, Emitter
    (`GameplayStatics.SpawnEmitterAtLocation` "/Game/StarterContent/Particles/P_Smoke.P_Smoke" _location _rotation _returnvalue)
    (`GameplayStatics.SpawnEmitterAtLocation` "/Game/StarterContent/Particles/P_Explosion.P_Explosion" _location _rotation _returnvalue)
    ; If there is a Remnant Sprite
    (if (== _remnant_sprite null)
      ; Show Remnant Sprite
      (`SceneComponent.SetVisibility` _remnant_sprite true false))
    ; Wait for Flipbook Animation to Finish
    (`KismetSystemLibrary.Delay` (`PaperFlipbookComponent.GetFlipbookLength` _destroyanimation))
    (`SceneComponent.SetVisibility` _destroyanimation false false)
    (`self.K2_DestroyActor`)
    (else
      (`KismetSystemLibrary.PrintString` (`KismetStringLibrary.BuildString_Double` "Damage to Building:" "" _output_get)))))

(event `self.ReceiveTick`
  (params (DeltaSeconds :type "Float (single-precision)"))
  (if (`self.PlayerHoots`)
    _))

(event `self.ReceiveBeginPlay`
  (bind _perchsize (`self.PerchSize`))
  (bind (_origin _boxextent) (`KismetSystemLibrary.GetComponentBounds` (`self.Intact_Sprite`)))
  (`|SpawnActorFromClass` "/Game/Blueprints/BP_Perch.BP_Perch_C" (`KismetMathLibrary.MakeTransform` (`KismetMathLibrary.MakeVector` (.x _origin) 0.0 (- (+ (.z _boxextent) (.z _origin)) 3.0)) (struct) (`KismetMathLibrary.MakeVector` _perchsize _perchsize _perchsize)) "Undefined" "MultiplyWithRoot" null null)
  ; Critter Spawns
  (set `self.CritterSpawnTime` (`KismetMathLibrary.RandomFloatInRange` 15.0 90.0) :!label _label)
  (`KismetSystemLibrary.Delay` (`self.CritterSpawnTime`))
  (`|SpawnActorFromClass` "/Game/Blueprints/Critters/BP_Critter.BP_Critter_C" (`KismetMathLibrary.MakeTransform` (`KismetMathLibrary.MakeVector` (.x (.location (`self.GetTransform`))) 0.0 (.z (.location (`self.GetTransform`))))) "Undefined" "MultiplyWithRoot" null null)
  (goto _label))

(event `HootHeard`
  ; Hoot Heard
  (`|SpawnActorFromClass` "/Game/Blueprints/Critters/BP_Critter.BP_Critter_C" (`KismetMathLibrary.MakeTransform` (`KismetMathLibrary.MakeVector` (.x (`SceneComponent.K2_GetComponentLocation` (`self.DefaultSceneRoot`))) 0.0 (.z (`SceneComponent.K2_GetComponentLocation` (`self.DefaultSceneRoot`))))) "Undefined" "MultiplyWithRoot" null null)
  (`KismetSystemLibrary.PrintString` "Critter Spawned by Hoot"))

(fn `UserConstructionScript`)