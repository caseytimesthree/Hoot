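; Bone structure building that scatters destructible buildings over its sprite and is destroyed once they are all gone.
; On BeginPlay it fires randomized line traces across the sprite bounds, one per BuildingCount.
; Each hit on a "BuildingBone"-tagged component spawns a randomly scaled BP_SpawnedBuilding that references this bone as its spawner.
; SpawnedBuildingDestroyed removes buildings from the tracked list, triggering an explosion and self-destruction when it empties.
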(event `self.ReceiveBeginPlay`
  (bind _spawninglinelength (`self.SpawningLineLength`))
  (bind _yoffset (`self.YOffset`))
  (bind (_origin _boxextent) (`KismetSystemLibrary.GetComponentBounds` (`self.BoneStructureSprite`)))
  (bind _returnvalue (- (`self.BuildingCount`) 1))
  (bind _y (.y (`SceneComponent.K2_GetComponentLocation` (`self.BoneStructureSprite`))))
  (bind _x (.x _boxextent))
  (bind _x_2 (.x _origin))
  (bind _z (.z _origin))
  (bind _returnvalue_2 (* (.x (.scale (`self.GetTransform`))) (* (+ (`KismetMathLibrary.RandomFloat`) 1.0) (`self.SpawnedBuildingSize`))))
  (bind _returnvalue_3 (`KismetMathLibrary.RandomFloatInRange` (- _x_2 _x) (+ _x_2 _x)))
  (`self.EnableInput` (`GameplayStatics.GetPlayerController` 0))
  (`KismetArrayLibrary.Array_Clear` (`self.SpawnedBuildings`))
  (for _ (range (+ _returnvalue 1))
    ; Find Points on Spawning Structure
    (bind (_outhit _returnvalue_4) (`KismetSystemLibrary.LineTraceSingle` :`Start` (`KismetMathLibrary.MakeVector` _returnvalue_3 (+ _y _yoffset) (+ _z (* _spawninglinelength (`KismetMathLibrary.RandomFloat`)))) :`End` (`KismetMathLibrary.MakeVector` _returnvalue_3 (- _y _yoffset) (- _z (* _spawninglinelength (`KismetMathLibrary.RandomFloat`)))) :`TraceChannel` "TraceTypeQuery1" :`bIgnoreSelf` false))
    ; Spawn Buildings
    (if _returnvalue_4
      (bind (_bblockinghit _binitialoverlap _time _distance _location _impactpoint _normal _impactnormal _physmat _hitactor _hitcomponent) (`GameplayStatics.BreakHitResult` _outhit))
      (if (`ActorComponent.ComponentHasTag` _hitcomponent "BuildingBone")
        (if true
          (`KismetSystemLibrary.PrintString` "Trace Hit")
          (bind _returnvalue_5 (`|SpawnActorFromClass` "/Game/Buildings/BP_SpawnedBuilding.BP_SpawnedBuilding_C" (`KismetMathLibrary.MakeTransform` (`KismetMathLibrary.MakeVector` (.x _location) (+ (.y _location) (* _returnvalue -1) (`self.YOffset`)) (.z _location)) (`KismetMathLibrary.Conv_VectorToRotator` (`KismetMathLibrary.MakeVector` (`KismetMathLibrary.RandomFloatInRange` -25.0 25.0))) (`KismetMathLibrary.MakeVector` _returnvalue_2 3.0 _returnvalue_2)) "Undefined" "MultiplyWithRoot" null null))
          (`KismetSystemLibrary.PrintString` "Building Spawned")
          (`KismetArrayLibrary.Array_Add` (`self.SpawnedBuildings`) _returnvalue_5)
          (bind _asbp_spawned_building (cast `/Game/Buildings/BP_SpawnedBuilding` _returnvalue_5))
          (set `/Game/Buildings/BP_SpawnedBuilding.SpawnerBone` self _asbp_spawned_building)))
      (else
        (`KismetSystemLibrary.PrintString` "Trace Missed")))))

(event `SpawnedBuildingDestroyed`
  (bind _returnvalue (`KismetArrayLibrary.Array_Length` (`self.SpawnedBuildings`)))
  (`KismetArrayLibrary.Array_RemoveItem` (`self.SpawnedBuildings`) (`self.DestroyedBuilding`))
  (`KismetSystemLibrary.PrintString` (`KismetStringLibrary.BuildString_Int` "Spawned Building Destroyed" "Buildings left on Bone:" _returnvalue))
  (if (== _returnvalue 0)
    (`GameplayStatics.SpawnEmitterAtLocation` "/Game/StarterContent/Particles/P_Explosion.P_Explosion" (`self.K2_GetActorLocation`) (struct) (10.0 10.0 10.0))
    (`self.K2_DestroyActor`)))

(fn `UserConstructionScript`)