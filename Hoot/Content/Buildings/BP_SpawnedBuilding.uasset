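; Destructible 2D building that picks a random sprite and flip, then hosts BP_Beetle critters bound to its bounds.
; A beetle spawns at BeginPlay and after random delays via SpawnBeetle; retried line traces store random sprite points, unused for placement.
; Damage flashes red; zero health triggers an explosion and destruction flipbook, then destruction notifies the owning BP_Building_Bones.
; Overlaps nudge depth against Z-fighting; perch and hoot-critter logic is disconnected.
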(event `self.ReceiveBeginPlay`
  (bind _spritearray (`self.SpriteArray`))
  (bind (_origin _boxextent) (`KismetSystemLibrary.GetComponentBounds` (`self.Intact_Sprite`)))
  ; SETUP
  (if (not (> (`KismetMathLibrary.RandomFloat`) 0.5))
    (`self.K2_SetActorTransform` (`KismetMathLibrary.MakeTransform` (`SceneComponent.K2_GetComponentLocation` (`self.DefaultSceneRoot`)) (.rotation (`self.GetTransform`)) (`KismetMathLibrary.MakeVector` (* (.x (.scale (`self.GetTransform`))) -1.0) (.y (.scale (`self.GetTransform`))) (.z (.scale (`self.GetTransform`)))))))
  (`self.EnableInput` (`GameplayStatics.GetPlayerController` 0))
  ;; RandomSprite
  (`PaperSpriteComponent.SetSprite` (`self.Intact_Sprite`) (`|GetArrayItem` _spritearray (`KismetMathLibrary.RandomInteger` (- (`KismetArrayLibrary.Array_Length` _spritearray) 1))))
  (`self.GetRandomLocationOnSprite`)
  ;; Spawn Critter (Beetle Type)
  (set `self.SpriteColorBase` (`PaperSpriteComponent.SpriteColor` (`self.Intact_Sprite`)))
  (bind _returnvalue (`|SpawnActorFromClass` "/Game/Blueprints/Critters/BP_Beetle.BP_Beetle_C" (`KismetMathLibrary.MakeTransform` (`KismetMathLibrary.MakeVector` (.x (`self.K2_GetActorLocation`)) (+ (.y (`self.K2_GetActorLocation`)) 0.01) (.z (`self.K2_GetActorLocation`))) (struct) (0.7 0.7 0.7)) "Undefined" "MultiplyWithRoot" null null null))
  (bind _asbp_beetle (cast `/Game/Blueprints/Critters/BP_Beetle` _returnvalue))
  (set `/Game/Blueprints/Critters/BP_Beetle.TargetSurface` self _asbp_beetle)
  (set `/Game/Blueprints/Critters/BP_Beetle.BuildingOrigin` _origin _asbp_beetle)
  (set `/Game/Blueprints/Critters/BP_Beetle.BuildingBounds` _boxextent _asbp_beetle))

(event `self.ReceiveTick`
  (params (DeltaSeconds :type "Float (single-precision)"))
  (set `self.SpriteYPosition` (.y (`SceneComponent.K2_GetComponentLocation` (`self.Intact_Sprite`)))))

(event `GetRandomLocationOnSprite`
  (bind _spawninglinelength (`self.SpawningLineLength`))
  (bind (_origin _boxextent) (`KismetSystemLibrary.GetComponentBounds` (`self.Intact_Sprite`)))
  (bind _x (.x _origin))
  (bind _z (.z _origin))
  (bind _x_2 (.x _boxextent))
  (bind _returnvalue (`KismetMathLibrary.RandomFloatInRange` (- _x _x_2) (+ _x _x_2)))
  ; Spawning Logic
  ;; Find Points on Spawning Structure
  (bind (_outhit _returnvalue_2) (`KismetSystemLibrary.LineTraceSingle` :`Start` (`KismetMathLibrary.MakeVector` _returnvalue 0.0 (+ _z (* _spawninglinelength (`KismetMathLibrary.RandomFloat`)))) :`End` (`KismetMathLibrary.MakeVector` _returnvalue 0.0 (- _z (* _spawninglinelength (`KismetMathLibrary.RandomFloat`)))) :`TraceChannel` "TraceTypeQuery1" :`bIgnoreSelf` false :!label _label))
  ;; RandomSpotonSprite
  (if _returnvalue_2
    (set `self.RandomLocationOnSprite` (`.Location` (`GameplayStatics.BreakHitResult` _outhit)))
    (else
      (goto _label))))

(event `DamageFX`
  ; Damage and health
  (`PaperSpriteComponent.SetSpriteColor` (`self.Intact_Sprite`) (make `LinearColor` 1.0 0.0 0.0 1.0))
  (`KismetSystemLibrary.Delay` 0.1)
  (`PaperSpriteComponent.SetSpriteColor` (`self.Intact_Sprite`) (`self.SpriteColorBase`)))

(event `self.ReceiveAnyDamage`
  (params (Damage :type "Float (single-precision)") (DamageType :type "DamageType Object Reference") (InstigatedBy :type "Controller Object Reference") (DamageCauser :type "Actor Object Reference"))
  (bind _destroyedemittersize (`self.DestroyedEmitterSize`))
  (bind _remnant_sprite (`self.Remnant_Sprite`))
  (bind _destroyanimation (`self.DestroyAnimation`))
  ; Damage and health
  ;; Receive Damage
  (`self.DamageFX`)
  (set `self.Health` (- (`self.Health`) Damage))
  (if (<= (`self.Health`) 0.0)
    ;; Remove Intact Sprite
    (`SceneComponent.SetVisibility` (`self.Intact_Sprite`) false false)
    ;; Play Destroy Animation
    (`SceneComponent.SetHiddenInGame` _destroyanimation false false)
    (`PaperFlipbookComponent.PlayFromStart` _destroyanimation)
    (`GameplayStatics.SpawnEmitterAtLocation` "/Game/StarterContent/Particles/P_Explosion.P_Explosion" (.location (`self.GetTransform`)) (.rotation (`self.GetTransform`)) (* (`KismetMathLibrary.MakeVector` _destroyedemittersize 0.0 _destroyedemittersize) (.scale (`self.GetTransform`))))
    ;; If there is a Remnant Sprite
    (if (== _remnant_sprite null)
      ;; Show Remnant Sprite
      (`SceneComponent.SetVisibility` _remnant_sprite true false))
    ;; Wait for Flipbook Animation to Finish
    (`KismetSystemLibrary.Delay` (`PaperFlipbookComponent.GetFlipbookLength` _destroyanimation))
    (`SceneComponent.SetVisibility` _destroyanimation false false)
    (`self.K2_DestroyActor`)))

(event `self.ReceiveActorBeginOverlap`
  (params (OtherActor :type "Actor Object Reference"))
  ; Offset Y to prevent Z Fighting
  (if (== OtherActor "BP_SpawnedBuilding")
    (`self.K2_SetActorLocation` (`KismetMathLibrary.MakeVector` (.x (`self.K2_GetActorLocation`)) (- (.y (`self.K2_GetActorLocation`)) 0.1) (.z (`self.K2_GetActorLocation`))))
    (`KismetSystemLibrary.PrintString` "Building Nudged")))

(event `self.ReceiveDestroyed`
  ; BuildingDestroyed
  (bind _asbp_building_bones (cast `/Game/Buildings/BP_Building_Bones` (`self.SpawnerBone`)))
  (set `/Game/Buildings/BP_Building_Bones.DestroyedBuilding` self _asbp_building_bones)
  (`/Game/Buildings/BP_Building_Bones.SpawnedBuildingDestroyed` _asbp_building_bones))

(event `SpawnBeetle`
  (bind (_origin _boxextent) (`KismetSystemLibrary.GetComponentBounds` (`self.Intact_Sprite`)))
  (bind _returnvalue (* (`KismetMathLibrary.RandomFloat`) (`self.BeetleSpawnRate`)))
  (`KismetSystemLibrary.PrintString` (`KismetStringLibrary.BuildString_Double` "" "Beetle Spawning in:" _returnvalue " Seconds"))
  (`KismetSystemLibrary.Delay` _returnvalue)
  ; Spawn Critter (Beetle Type)
  (`self.GetRandomLocationOnSprite`)
  (bind _returnvalue_2 (`|SpawnActorFromClass` "/Game/Blueprints/Critters/BP_Beetle.BP_Beetle_C" (`KismetMathLibrary.MakeTransform` (`KismetMathLibrary.MakeVector` (.x (`self.K2_GetActorLocation`)) (+ (.y (`self.K2_GetActorLocation`)) 0.01) (.z (`self.K2_GetActorLocation`))) (struct) (0.7 0.7 0.7)) "Undefined" "MultiplyWithRoot" null null null))
  (bind _asbp_beetle (cast `/Game/Blueprints/Critters/BP_Beetle` _returnvalue_2))
  (set `/Game/Blueprints/Critters/BP_Beetle.TargetSurface` self _asbp_beetle)
  (set `/Game/Blueprints/Critters/BP_Beetle.BuildingOrigin` _origin _asbp_beetle)
  (set `/Game/Blueprints/Critters/BP_Beetle.BuildingBounds` _boxextent _asbp_beetle)
  (`KismetSystemLibrary.PrintString` "Beetle Spawned"))

(event `HootHeard`
  ; Redacted
  ;; HootHeard
)

(fn `UserConstructionScript`)