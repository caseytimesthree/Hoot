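; Owl nest actor that tracks the satiation of three chicks, which perish if left unfed.
; On BeginPlay it registers itself with BP_Owl and Hoot_PlayerController, stores its Y position and starts a randomized Delay loop per chick.
; Each loop lowers that chick's Hunger value, where zero means starving, then hides the chick and notifies UI_Hunger.
; Separate Feed events restore the value and count feedings.
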(event `self.ReceiveBeginPlay`
  (`self.HungerDescreaseChick1`)
  (`self.Chick2HungerDecrease`)
  (`self.Chick3HungerDescrease`)
  (bind _asbp_owl (cast `/Game/Owl/BP_Owl` (`GameplayStatics.GetPlayerPawn` 0)))
  (set `/Game/Owl/BP_Owl.NestObject` self _asbp_owl)
  (bind _ashoot_player_controller (cast `/Game/Owl/Hoot_PlayerController` (`GameplayStatics.GetPlayerController` 0)))
  (set `/Game/Owl/Hoot_PlayerController.NestObject` self _ashoot_player_controller)
  (set `self.SpriteYPosition` (.y (`SceneComponent.K2_GetComponentLocation` (`self.Nest`)))))

(event `self.ReceiveTick`
  (params (DeltaSeconds :type "Float (single-precision)")))

(event `HungerDescreaseChick1`
  (bind _chick1hunger (`self.Chick1Hunger`))
  ; Chick 1 Hunger
  (`KismetSystemLibrary.Delay` (+ (`self.ChickHungerTime`) (`KismetMathLibrary.RandomFloatInRange` -3.0 3.0)) :!label _label)
  (if (< _chick1hunger 0.01)
    (`SceneComponent.SetVisibility` (`self.Chick1`) false false)
    (`KismetSystemLibrary.PrintString` "Chick 1 Perished!")
    (bind _asui_hunger (cast `/Game/UI/UI_Hunger` (`self.UIHungerObject`)))
    (`/Game/UI/UI_Hunger.Chick1Perished` _asui_hunger)
    (elif (> _chick1hunger 0.0)
      (bind _output_get (set `self.Chick1Hunger` (`KismetMathLibrary.FClamp` (- (`self.Chick1Hunger`) 0.2))))
      (`KismetSystemLibrary.PrintString` (`KismetStringLibrary.BuildString_Double` "Chich Hunger Increased" "Chick 1 Satiation:" _output_get))
      (goto _label))))

(event `FeedChick1`
  ; Feed Chick 1
  (set `self.Chick1Hunger` (`KismetMathLibrary.FClamp` (+ (`self.Chick1Hunger`) 0.5)))
  (set `self.Chick1FedAmt` (+ (`self.Chick1FedAmt`) 1)))

(event `Chick2HungerDecrease`
  (bind _chick2hunger (`self.Chick2Hunger`))
  ; Chick 2 Hunger
  (`KismetSystemLibrary.Delay` (+ (`self.ChickHungerTime`) (`KismetMathLibrary.RandomFloatInRange` -3.0 3.0)) :!label _label_2)
  (if (< _chick2hunger 0.01)
    (`SceneComponent.SetVisibility` (`self.Chick2`) false false)
    (`KismetSystemLibrary.PrintString` "Chick 2 Perished!")
    (bind _asui_hunger (cast `/Game/UI/UI_Hunger` (`self.UIHungerObject`)))
    (`/Game/UI/UI_Hunger.Chick2Perished` _asui_hunger)
    (elif (> _chick2hunger 0.0)
      (bind _output_get (set `self.Chick2Hunger` (`KismetMathLibrary.FClamp` (- _chick2hunger 0.2))))
      (`KismetSystemLibrary.PrintString` (`KismetStringLibrary.BuildString_Double` "Chich Hunger Increased" "Chick 2 Satiation:" _output_get))
      (goto _label_2))))

(event `FeedChick2`
  ; FeedChick2
  (set `self.Chick2Hunger` (`KismetMathLibrary.FClamp` (+ (`self.Chick2Hunger`) 0.5)))
  (set `self.Chick2FedAmt` (+ (`self.Chick2FedAmt`) 1)))

(event `Chick3HungerDescrease`
  (bind _chick3hunger (`self.Chick3Hunger`))
  ; Chick 3 Hunger
  (`KismetSystemLibrary.Delay` (+ (`self.ChickHungerTime`) (`KismetMathLibrary.RandomFloatInRange` -3.0 3.0)) :!label _label_3)
  (if (< _chick3hunger 0.01)
    (`SceneComponent.SetVisibility` (`self.Chick3`) false false)
    (`KismetSystemLibrary.PrintString` "Chick 3 Perished!")
    (bind _asui_hunger (cast `/Game/UI/UI_Hunger` (`self.UIHungerObject`)))
    (`/Game/UI/UI_Hunger.Chick3Perished` _asui_hunger)
    (elif (> _chick3hunger 0.0)
      (bind _output_get (set `self.Chick3Hunger` (`KismetMathLibrary.FClamp` (- _chick3hunger 0.2))))
      (`KismetSystemLibrary.PrintString` (`KismetStringLibrary.BuildString_Double` "Chich Hunger Increased" "Chick 3 Satiation:" _output_get))
      (goto _label_3))))

(event `FeedChick3`
  ; FeedChick3
  (set `self.Chick3Hunger` (`KismetMathLibrary.FClamp` (+ (`self.Chick3Hunger`) 0.5)))
  (set `self.Chick3FedAmt` (+ (`self.Chick3FedAmt`) 1)))

(fn `UserConstructionScript`)