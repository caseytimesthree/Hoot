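; Owl actor that flies toward a target location or dives at a critter target, switching between flying and diving visuals.
; Each Tick interpolates X and Z with a swept move, applying a dive speed multiplier while IsDiving, which is not set in this graph.
; Diving resets TargetLocation to the current position; the arrival check (distance below zero) never passes, so IsMoving stays true otherwise.
; Capsule hits only print a debug message.
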(event `self.ReceiveBeginPlay`
  (set `self.IsCarrying` false)
  (`SceneComponent.SetVisibility` (`self.Idle`) false false)
  (`SceneComponent.SetVisibility` (`self.Diving`) false false)
  (`SceneComponent.SetVisibility` (`self.Flying`) true false)
  (set `self.TargetLocation` (`self.K2_GetActorLocation`)))

(event `self.ReceiveTick`
  (params (DeltaSeconds :type "Float (single-precision)"))
  (bind (_returnvalue_x _returnvalue_y _returnvalue_z) (`KismetMathLibrary.BreakVector` (`KismetMathLibrary.VInterpTo` (`self.K2_GetActorLocation`) (`self.TargetLocation`) DeltaSeconds (* (`self.MovementSpeed`) DeltaSeconds))))
  (bind _returnvalue (`KismetMathLibrary.Distance2D` (`KismetMathLibrary.Conv_VectorToVector2D` (`self.TargetLocation`)) (`KismetMathLibrary.Conv_VectorToVector2D` (`self.K2_GetActorLocation`))))
  (if (`self.isDiving`)
    (set `self.TargetLocation` (`self.K2_GetActorLocation`))
    (`SceneComponent.SetVisibility` (`self.Flying`) false false)
    (`SceneComponent.SetVisibility` (`self.Diving`) true false)
    (`self.K2_SetActorLocation` (`KismetMathLibrary.MakeVector` (.x (`KismetMathLibrary.VInterpTo` (`self.K2_GetActorLocation`) (`self.CritterTarget`) DeltaSeconds (* (`self.MovementSpeed`) (* DeltaSeconds (`self.CritterDiveSpeedMultiplier`))))) 0.0 (.z (`KismetMathLibrary.VInterpTo` (`self.K2_GetActorLocation`) (`self.CritterTarget`) DeltaSeconds (* (`self.MovementSpeed`) (* DeltaSeconds (`self.CritterDiveSpeedMultiplier`)))))) true)
    (else
      (`SceneComponent.SetVisibility` (`self.Flying`) true false)
      (`SceneComponent.SetVisibility` (`self.Diving`) false false)
      (if (< _returnvalue 0.0)
        (`KismetSystemLibrary.PrintString` (`KismetStringLibrary.BuildString_Double` "DISTANCE =")))
      (if (< _returnvalue 0.0)
        (set `self.bIsMoving` false)
        (else
          (set `self.bIsMoving` true)
          (`self.K2_SetActorLocation` (`KismetMathLibrary.MakeVector` _returnvalue_x 0.0 _returnvalue_z) true))))))

(event `self.Capsule.OnComponentHit`
  (params (HitComponent :type "PrimitiveComponent Object Reference") (OtherActor :type "Actor Object Reference") (OtherComp :type "PrimitiveComponent Object Reference") (NormalImpulse :type "Vector Structure") (Hit :type "HitResult Structure (by ref)"))
  (`KismetSystemLibrary.PrintString` "Owl Collided with something"))

(fn `UserConstructionScript`)